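; BP_Gem is a collectable pickup that spins via a timeline and counts toward unlocking the exit door.
; The first sphere overlap by BP_FirstPersonCharacter plays a sound, increments and flashes the WBP_GemUI counter, then hides and later destroys the gem.
; The count lives in widget text; when it matches GemsNeeded, the first BP_ExitDoor found becomes active and turns green.
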(event OnComponentBeginOverlap(Sphere)
  (params (OverlappedComponent :type Primitive%20Component%20Object%20Reference) (OtherActor :type Actor%20Object%20Reference) (OtherComp :type Primitive%20Component%20Object%20Reference) (OtherBodyIndex :type Integer) (bFromSweep :type Boolean) (SweepResult :type Hit%20Result%20Structure%20%28by%20ref%29))
  (Utilities|Casting|CastToBP_FirstPersonCharacter OtherActor)
  (Utilities|FlowControl|DoOnce false
    (:Completed
      (Audio|PlaySoundatLocation "/Game/Collectables/Sounds/GotGem.GotGem" "0, 0, 0" "0, 0, 0" 1.0 1.0 0.0 0 0 0 0)
      (bind _foundwidgets (Widget|GetAllWidgetsOfClass "/Game/UIElements/WBP_GemUI.WBP_GemUI_C" true))
      (CallFunction|IncrementGem (Utilities|Array|Get(acopy) _foundwidgets))
      (CallFunction|HandleFlash (Utilities|Array|Get(acopy) _foundwidgets) (Utilities|Array|Get(acopy) _foundwidgets))
      (CallFunction|HandleCountGem (Utilities|Array|Get(acopy) _foundwidgets) (Utilities|Array|Get(acopy) _foundwidgets))
      (Rendering|SetActorHiddenInGame true)
      (Utilities|FlowControl|Delay 2.0)
      (Actor|DestroyActor))))

(event EventBeginPlay
  (bind _newtrack_0 (Timeline|Sequence Play)
    (:Update
      (Transformation|SetWorldRotation (Variables|Default|GetSphere1) (Math|Rotator|MakeRotator 0.0 _newtrack_0 _newtrack_0) false false))))

(event Collision|EventActorBeginOverlap
  (params (OtherActor :type Actor%20Object%20Reference)))

(event EventTick
  (params (DeltaSeconds :type Float%20%28single-precision%29)))

(fn ConstructionScript)

(fn IncrementGem
  (params (self2 :type WBP%20Gem%20UI%20Object%20Reference))
  (bind _gemscollected (Variables|/Game/UIElements/WBP_GemUI.WBP_GemUI_C|GetGemsCollected self2))
  (bind _returnvalue (Class|TextBlock|GetText _gemscollected))
  (Development|PrintText _returnvalue)
  (bind _result (Math|Integer|IncrementInt (Math|Conversions|ToInteger(Byte) (Utilities|String|ToString(Text) _returnvalue)))
    (:%20%20
      (Rendering|Components|TextRender|SetText _gemscollected (Utilities|Text|ToText(Integer) _result)))))

(fn HandleCountGem
  (params (self2 :type WBP%20Gem%20UI%20Object%20Reference) (self3 :type WBP%20Gem%20UI%20Object%20Reference))
  (if (Utilities|Enum|Equal(Enum) (Class|TextBlock|GetText (Variables|/Game/UIElements/WBP_GemUI.WBP_GemUI_C|GetGemsCollected self3)) (Class|TextBlock|GetText (Variables|/Game/UIElements/WBP_GemUI.WBP_GemUI_C|GetGemsNeeded self2)))
    (bind _outactors (Actor|GetAllActorsOfClass "/Game/Door/BP_ExitDoor.BP_ExitDoor_C"))
    (Variables|/Game/Door/BP_ExitDoor.BP_ExitDoor_C|SetisActive (Utilities|Array|Get(acopy) _outactors) true)
    (Rendering|Material|SetMaterial (Variables|/Game/Door/BP_ExitDoor.BP_ExitDoor_C|GetDoor (Utilities|Array|Get(acopy) _outactors)) 0 "/Game/Door/M_DoorGreen.M_DoorGreen")))

(fn HandleFlash
  (params (self2 :type WBP%20Gem%20UI%20Object%20Reference) (self3 :type User%20Widget%20Object%20Reference))
  (UserInterface|Animation|PlayAnimation self3 (Variables|/Game/UIElements/WBP_GemUI.WBP_GemUI_C|GetFlash self2) 0.0 1 "Forward" 1.0 false))