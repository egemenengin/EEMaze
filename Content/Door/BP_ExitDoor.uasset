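; BP_ExitDoor is an exit trigger that moves the player to the next level.
; When BP_FirstPersonCharacter first overlaps its Box, a DoOnce fires and checks IsActive.
; If active, it shows a WBP_Fade widget, plays its Fade animation in reverse, then opens NextLevel after a short delay.
; The DoOnce precedes the IsActive check, so an overlap while inactive also consumes it.
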(event OnComponentBeginOverlap(Box)
  (params (OverlappedComponent :type Primitive%20Component%20Object%20Reference) (OtherActor :type Actor%20Object%20Reference) (OtherComp :type Primitive%20Component%20Object%20Reference) (OtherBodyIndex :type Integer) (bFromSweep :type Boolean) (SweepResult :type Hit%20Result%20Structure%20%28by%20ref%29))
  (Utilities|Casting|CastToBP_FirstPersonCharacter OtherActor)
  (Utilities|FlowControl|DoOnce false
    (:Completed
      (if (Variables|Default|GetisActive)
        (bind _returnvalue (UserInterface|CreateWidget "/Game/UIElements/WBP_Fade.WBP_Fade_C"))
        (UserInterface|Viewport|AddtoViewport _returnvalue 0)
        (UserInterface|Animation|PlayAnimation _returnvalue (Variables|/Game/UIElements/WBP_Fade.WBP_Fade_C|GetFade _returnvalue) 0.0 1 "Reverse" 1.0 false)
        (Utilities|FlowControl|Delay 0.4)
        (Game|OpenLevel(byName) (Variables|Default|GetNextLevel))))))

(event EventBeginPlay)

(event Collision|EventActorBeginOverlap
  (params (OtherActor :type Actor%20Object%20Reference)))

(event EventTick
  (params (DeltaSeconds :type Float%20%28single-precision%29)))

(fn ConstructionScript)